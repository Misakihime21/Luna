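; Bathroom light switch actor that toggles matching lights and triggers a one-time bathroom demon vanish.
; Interaction flips the switch via a timeline with a click sound.
; If the demon exists, its first trigger destroys it with a whoosh, then briefly shows a Luna monologue widget.
; Outside the game mode's SearchMode, it toggles lights sharing its LightIndex and resets the DoOnce interaction gate, which otherwise stays closed.
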(event `self.ReceiveBeginPlay`
  (bind _asbp_lgamemode_first_person (cast `/Game/Luna/Blueprints/GameMode/BP_LGamemodeFirstPerson` (`GameplayStatics.GetGameMode`)))
  (set `self.As BP LGamemode First Person` _asbp_lgamemode_first_person)
  (bind _returnvalue (`GameplayStatics.GetActorOfClass` "/Game/Luna/Blueprints/BP_DemonBathroom.BP_DemonBathroom_C"))
  (set `self.As DemonBathroom` _returnvalue)
  (bind _outactors (`GameplayStatics.GetAllActorsOfClass` "/Game/Luna/LightSwitch/BP_Light.BP_Light_C"))
  (for _array_element _outactors
    (`KismetArrayLibrary.Array_Add` (`self.LightsArray`) _array_element)))

(event `FlipFlop`
  (`GameplayStatics.PlaySoundAtLocation` "/Game/Luna/Sounds/mixkit-classic-click-1117.mixkit-classic-click-1117" (`SceneComponent.K2_GetComponentLocation` (`self.lightswitch_CoverPlate_001`)) (struct) 1.0 1.0 0.0 null null null null)
  (`/Engine/EditorBlueprintResources/StandardMacros.FlipFlop`
    (:`A`
      (bind (_direction _switchalpha) (`Timeline|Timeline_0` :!label _label)
        (:`Update`
          (`SceneComponent.K2_SetRelativeRotation` (`self.lightswitch_Switch_001`) (`KismetMathLibrary.MakeRotator` 0.0 (`KismetMathLibrary.Lerp` 0.0 -10.0 _switchalpha)) false false))))
    (:`B`
      (goto _label :!via `Reverse`))))

(event `Demon`
  ;[1 0.2241 0.1643] Bathroom Demon
  (`self.As DemonBathroom`
    (:`then`
      (`/Engine/EditorBlueprintResources/StandardMacros.DoOnce` false
        (:`Completed`
          (`GameplayStatics.PlaySoundAtLocation` "/Game/Luna/Sounds/mixkit-quick-air-woosh-2605.mixkit-quick-air-woosh-2605" (`SceneComponent.K2_GetComponentLocation` (`/Game/Luna/Blueprints/BP_DemonBathroom.Eye` (`self.As DemonBathroom`))) (struct) 1.0 1.0 0.0 null null null null)
          (`self.K2_DestroyActor` (`self.As DemonBathroom`))
          (`KismetSystemLibrary.Delay` 2.0)
          (bind _returnvalue (`|CreateWidget` "/Game/Luna/UI/WPB_LunaMonologue.WPB_LunaMonologue_C" (`GameplayStatics.GetPlayerController` 0) (`self.Luna Says`)))
          (`UserWidget.AddToViewport` _returnvalue 0)
          (`KismetSystemLibrary.Delay` 2.0)
          (`Widget.RemoveFromParent` _returnvalue))))
    (:`else`)))

(event `/Game/Luna/Input/BPI_Interactive.Interactive`
  (`/Engine/EditorBlueprintResources/StandardMacros.DoOnce` false :!label _label_2
    (:`Completed`
      (`self.FlipFlop`)
      (`self.Demon`)
      (if (not (`/Game/Luna/Blueprints/GameMode/BP_LGamemodeFirstPerson.SearchMode` (`self.As BP LGamemode First Person`)))
        (for _array_element (`self.LightsArray`)
          (if (== (`/Game/Luna/LightSwitch/BP_Light.Light Index` _array_element) (`self.Light Index`))
            (message `/Game/Luna/LightSwitch/BPI_LightsInterface.Toggle Lights` _array_element)
            (goto _label_2 :!via `Reset`)
            (else
              (goto _label_2 :!via `Reset`))))))))

(fn `UserConstructionScript`)