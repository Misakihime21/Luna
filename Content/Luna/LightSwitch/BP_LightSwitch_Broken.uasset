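; BP_LightSwitch_Broken is an interactable broken light switch that clicks and moves without controlling any light, while Luna comments on it.
; Interactive toggles the switch through FlipFlop, playing a click sound and running a timeline forward or in reverse to tilt the switch mesh.
; It also shows a Luna monologue widget briefly, with a DoOnce that resets after the delay to block repeat presses.
; BeginPlay caches the first-person game mode, which these graphs never use.
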(event `self.ReceiveBeginPlay`
  (bind _asbp_lgamemode_first_person (cast `/Game/Luna/Blueprints/GameMode/BP_LGamemodeFirstPerson` (`GameplayStatics.GetGameMode`)))
  (set `self.As BP LGamemode First Person` _asbp_lgamemode_first_person))

(event `FlipFlop`
  (`GameplayStatics.PlaySoundAtLocation` "/Game/Luna/Sounds/mixkit-classic-click-1117.mixkit-classic-click-1117" (`SceneComponent.K2_GetComponentLocation` (`self.lightswitch_CoverPlate_001`)) (struct) 1.0 1.0 0.0 null null null null)
  (`/Engine/EditorBlueprintResources/StandardMacros.FlipFlop`
    (:`A`
      (bind (_direction _switchalpha) (`Timeline|Timeline_0` :!label _label)
        (:`Update`
          (`SceneComponent.K2_SetRelativeRotation` (`self.lightswitch_Switch_001`) (`KismetMathLibrary.MakeRotator` 0.0 (`KismetMathLibrary.Lerp` 0.0 -10.0 _switchalpha)) false false))))
    (:`B`
      (goto _label :!via `Reverse`))))

(event `/Game/Luna/Input/BPI_Interactive.Interactive`
  (`/Engine/EditorBlueprintResources/StandardMacros.DoOnce` false :!label _label_2
    (:`Completed`
      (`self.FlipFlop`)
      (bind _returnvalue (`|CreateWidget` "/Game/Luna/UI/WPB_LunaMonologue.WPB_LunaMonologue_C" (`GameplayStatics.GetPlayerController` 0) (`self.Luna Says`)))
      (`UserWidget.AddToViewport` _returnvalue 0)
      (`KismetSystemLibrary.Delay` 3.0)
      (`Widget.RemoveFromParent` _returnvalue)
      (goto _label_2 :!via `Reset`))))

(fn `UserConstructionScript`)