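; BP_Light is a point light actor that can be toggled on and off at runtime.
; The construction script applies the IsOn state, color and intensity variables to the PointLight component, so the configured look shows at placement.
; The ToggleLights event flips IsOn and updates the component's visibility to match.
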(event `/Game/Luna/LightSwitch/BPI_LightsInterface.Toggle Lights`
  (bind _output_get (set `self.IsOn` (not (`self.IsOn`))))
  (`SceneComponent.SetVisibility` (`self.PointLight`) _output_get false))

(fn `UserConstructionScript`
  (bind _pointlight (`self.PointLight`))
  (`SceneComponent.SetVisibility` (`self.PointLight`) (`self.IsOn`) false)
  (`LightComponent.SetLightColor` _pointlight (`self.New Light Color`) true)
  (`LightComponent.SetIntensity` _pointlight (`self.New Intensity`)))