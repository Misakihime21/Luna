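; BP_MomSleeping is a one-shot story trigger that fires when the Luna character overlaps its Collision component.
; It casts the game mode to BP_LGamemodeFirstPerson, enables SearchMode and drives four Luna lines by setting LunaSays before each call.
; Midway through the lines it turns off all lights through the game mode and plays a 2D sound.
; The actor destroys itself after a delay once the sequence has run.
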(event `self.Collision.OnComponentBeginOverlap`
  (params (OverlappedComponent :type "PrimitiveComponent Object Reference") (OtherActor :type "Actor Object Reference") (OtherComp :type "PrimitiveComponent Object Reference") (OtherBodyIndex :type Integer) (bFromSweep :type Boolean) (SweepResult :type "HitResult Structure (by ref)"))
  (cast `/Game/Luna/Blueprints/BP_LunaCharacter` OtherActor)
  (`/Engine/EditorBlueprintResources/StandardMacros.DoOnce` false
    (:`Completed`
      (bind _asbp_lgamemode_first_person (cast `/Game/Luna/Blueprints/GameMode/BP_LGamemodeFirstPerson` (`GameplayStatics.GetGameMode`)))
      (set `/Game/Luna/Blueprints/GameMode/BP_LGamemodeFirstPerson.SearchMode` true _asbp_lgamemode_first_person)
      (set `/Game/Luna/Blueprints/GameMode/BP_LGamemodeFirstPerson.Luna Says` (`self.Luna Says`) _asbp_lgamemode_first_person)
      (`/Game/Luna/Blueprints/GameMode/BP_LGamemodeFirstPerson.LunaSays` _asbp_lgamemode_first_person)
      (set `/Game/Luna/Blueprints/GameMode/BP_LGamemodeFirstPerson.Luna Says` (`self.Luna Says_2`) _asbp_lgamemode_first_person)
      (`/Game/Luna/Blueprints/GameMode/BP_LGamemodeFirstPerson.LunaSays` _asbp_lgamemode_first_person)
      (`/Game/Luna/Blueprints/GameMode/BP_LGamemodeFirstPerson.TurnOffALLLights` _asbp_lgamemode_first_person)
      (`GameplayStatics.PlaySound2D` null 1.0 1.0 0.0 null null)
      (set `/Game/Luna/Blueprints/GameMode/BP_LGamemodeFirstPerson.Luna Says` (`self.Luna Says_3`) _asbp_lgamemode_first_person)
      (`/Game/Luna/Blueprints/GameMode/BP_LGamemodeFirstPerson.LunaSays` _asbp_lgamemode_first_person)
      (set `/Game/Luna/Blueprints/GameMode/BP_LGamemodeFirstPerson.Luna Says` (`self.Luna Says_4`) _asbp_lgamemode_first_person)
      (`/Game/Luna/Blueprints/GameMode/BP_LGamemodeFirstPerson.LunaSays` _asbp_lgamemode_first_person)
      (`KismetSystemLibrary.Delay` 30.0)
      (`self.K2_DestroyActor`))))

(fn `UserConstructionScript`)