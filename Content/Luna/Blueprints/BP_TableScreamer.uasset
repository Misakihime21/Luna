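; BP_TableScreamer is a one-shot jump scare built around a coffee table, triggered by BP_LunaCharacter.
; Overlapping CollisionSuspence plays a suspense swell at the table.
; Overlapping CollisionScreamer starts a Timeline that lifts the table, then after a delay plays a collapse sound, destroys it and reveals the broken version.
; It then passes LunaSays to BP_LGamemodeFirstPerson and calls its LunaSays.
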(event `self.CollisionSuspence.OnComponentBeginOverlap`
  (params (OverlappedComponent :type "PrimitiveComponent Object Reference") (OtherActor :type "Actor Object Reference") (OtherComp :type "PrimitiveComponent Object Reference") (OtherBodyIndex :type Integer) (bFromSweep :type Boolean) (SweepResult :type "HitResult Structure (by ref)"))
  (cast `/Game/Luna/Blueprints/BP_LunaCharacter` OtherActor)
  (`/Engine/EditorBlueprintResources/StandardMacros.DoOnce` false
    (:`Completed`
      (`GameplayStatics.PlaySoundAtLocation` "/Game/Luna/Sounds/mixkit-cinematic-suspense-swell-786.mixkit-cinematic-suspense-swell-786" (`SceneComponent.K2_GetComponentLocation` (`self.SurpriseCoffeeTable`)) (struct) 1.0 1.0 0.0 null null null null))))

(event `self.CollisionScreamer.OnComponentBeginOverlap`
  (params (OverlappedComponent :type "PrimitiveComponent Object Reference") (OtherActor :type "Actor Object Reference") (OtherComp :type "PrimitiveComponent Object Reference") (OtherBodyIndex :type Integer) (bFromSweep :type Boolean) (SweepResult :type "HitResult Structure (by ref)"))
  (bind _surprisecoffeetable (`self.SurpriseCoffeeTable`))
  (cast `/Game/Luna/Blueprints/BP_LunaCharacter` OtherActor)
  (`/Engine/EditorBlueprintResources/StandardMacros.DoOnce` false
    (:`Completed`
      (`self.Moving`)
      (`KismetSystemLibrary.Delay` 1.0)
      (`GameplayStatics.PlaySoundAtLocation` "/Game/StarterContent/Audio/Collapse01.Collapse01" (`SceneComponent.K2_GetComponentLocation` _surprisecoffeetable) (struct) 1.0 1.0 0.0 null null null null)
      (`ActorComponent.K2_DestroyComponent` _surprisecoffeetable)
      (`SceneComponent.SetVisibility` (`self.SurpriseCoffeeTable_Broken`) true false)
      (bind _asbp_lgamemode_first_person (cast `/Game/Luna/Blueprints/GameMode/BP_LGamemodeFirstPerson` (`GameplayStatics.GetGameMode`)))
      (set `/Game/Luna/Blueprints/GameMode/BP_LGamemodeFirstPerson.Luna Says` (`self.Luna Says`) _asbp_lgamemode_first_person)
      (`/Game/Luna/Blueprints/GameMode/BP_LGamemodeFirstPerson.LunaSays` _asbp_lgamemode_first_person))))

(event `Moving`
  (bind _surprisecoffeetable (`self.SurpriseCoffeeTable`))
  (bind _returnvalue (`SceneComponent.K2_GetComponentLocation` _surprisecoffeetable))
  (bind (_direction _alpha) (`Timeline|Timeline`)
    (:`Update`
      (`SceneComponent.K2_SetRelativeLocation` _surprisecoffeetable (`KismetMathLibrary.VLerp` _returnvalue (+ _returnvalue (0.0 0.0 100.0)) _alpha) false false))))

(fn `UserConstructionScript`)