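; BP_PlateScreamer is a one-shot jump-scare prop: a plate that moves and breaks when the Luna character approaches.
; CollisionSuspence plays a thunder-and-rain sound at the plate.
; CollisionScreamer starts a Timeline that shifts the plate along Z, then after a short delay plays a thunder impact and swaps in the broken mesh.
; It then passes its LunaSays value to the first-person game mode and triggers that reaction.
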(event `self.CollisionSuspence.OnComponentBeginOverlap`
  (params (OverlappedComponent :type "PrimitiveComponent Object Reference") (OtherActor :type "Actor Object Reference") (OtherComp :type "PrimitiveComponent Object Reference") (OtherBodyIndex :type Integer) (bFromSweep :type Boolean) (SweepResult :type "HitResult Structure (by ref)"))
  (cast `/Game/Luna/Blueprints/BP_LunaCharacter` OtherActor)
  (`/Engine/EditorBlueprintResources/StandardMacros.DoOnce` false
    (:`Completed`
      (`GameplayStatics.PlaySoundAtLocation` "/Game/Luna/Sounds/mixkit-big-thunder-with-rain-1291.mixkit-big-thunder-with-rain-1291" (`SceneComponent.K2_GetComponentLocation` (`self.Plate`)) (struct) 1.0 1.0 0.0 null null null null))))

(event `self.CollisionScreamer.OnComponentBeginOverlap`
  (params (OverlappedComponent :type "PrimitiveComponent Object Reference") (OtherActor :type "Actor Object Reference") (OtherComp :type "PrimitiveComponent Object Reference") (OtherBodyIndex :type Integer) (bFromSweep :type Boolean) (SweepResult :type "HitResult Structure (by ref)"))
  (bind _plate (`self.Plate`))
  (cast `/Game/Luna/Blueprints/BP_LunaCharacter` OtherActor)
  (`/Engine/EditorBlueprintResources/StandardMacros.DoOnce` false
    (:`Completed`
      (`self.Moving`)
      (`KismetSystemLibrary.Delay` 0.5)
      (`GameplayStatics.PlaySoundAtLocation` "/Game/Luna/Sounds/mixkit-fast-thunder-impact-1279.mixkit-fast-thunder-impact-1279" (`SceneComponent.K2_GetComponentLocation` _plate) (struct) 1.0 1.0 0.5 null null null null)
      (`ActorComponent.K2_DestroyComponent` _plate)
      (`SceneComponent.SetVisibility` (`self.Plate_Broken`) true false)
      (bind _asbp_lgamemode_first_person (cast `/Game/Luna/Blueprints/GameMode/BP_LGamemodeFirstPerson` (`GameplayStatics.GetGameMode`)))
      (set `/Game/Luna/Blueprints/GameMode/BP_LGamemodeFirstPerson.Luna Says` (`self.Luna Says`) _asbp_lgamemode_first_person)
      (`/Game/Luna/Blueprints/GameMode/BP_LGamemodeFirstPerson.LunaSays` _asbp_lgamemode_first_person))))

(event `Moving`
  (bind _plate (`self.Plate`))
  (bind _returnvalue (`SceneComponent.K2_GetComponentLocation` _plate))
  (bind (_direction _alpha) (`Timeline|Timeline`)
    (:`Update`
      (`SceneComponent.K2_SetRelativeLocation` _plate (`KismetMathLibrary.VLerp` _returnvalue (+ _returnvalue (0.0 0.0 5.0)) _alpha) false false))))

(fn `UserConstructionScript`)