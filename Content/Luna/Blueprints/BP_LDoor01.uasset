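; BP_LDoor01 is an interactive door that swings open and closed around the yaw or roll of its DoorA component.
; Box overlap opens a gate for BP_LunaCharacter, only when the game mode is BP_LGamemodeFirstPerson, and closes it when the character leaves.
; While the gate is open, each Interactive event alternates a FlipFlop between playing and reversing a Timeline that lerps DoorA's relative rotation through 90 degrees.
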(event `/Game/Luna/Input/BPI_Interactive.Interactive`
  (`/Engine/EditorBlueprintResources/StandardMacros.Gate` true :!label _label
    (:`Exit`
      (`/Engine/EditorBlueprintResources/StandardMacros.FlipFlop`
        (:`A`
          (bind (_direction _alpha) (`Timeline|Timeline` :!label _label_2)
            (:`Update`
              (`SceneComponent.K2_SetRelativeRotation` (`self.Door_a`) (`KismetMathLibrary.RLerp` (struct) (struct :`Yaw` -90.0) _alpha) false false))))
        (:`B`
          (goto _label_2 :!via `Reverse`))))))

(event `self.Box.OnComponentBeginOverlap`
  (params (OverlappedComponent :type "PrimitiveComponent Object Reference") (OtherActor :type "Actor Object Reference") (OtherComp :type "PrimitiveComponent Object Reference") (OtherBodyIndex :type Integer) (bFromSweep :type Boolean) (SweepResult :type "HitResult Structure (by ref)"))
  (cast `/Game/Luna/Blueprints/BP_LunaCharacter` OtherActor)
  (cast `/Game/Luna/Blueprints/GameMode/BP_LGamemodeFirstPerson` (`GameplayStatics.GetGameMode`))
  (goto _label :!via `Open`))

(event `self.Box.OnComponentEndOverlap`
  (params (OverlappedComponent :type "PrimitiveComponent Object Reference") (OtherActor :type "Actor Object Reference") (OtherComp :type "PrimitiveComponent Object Reference") (OtherBodyIndex :type Integer))
  (cast `/Game/Luna/Blueprints/BP_LunaCharacter` OtherActor)
  (goto _label :!via `Close`))

(fn `UserConstructionScript`)