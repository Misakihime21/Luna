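; BP_Couch_Livingroom is the interactable living room couch that shows one of Luna's monologue lines when used.
; It caches the first-person game mode on BeginPlay, then picks the search or ending line from that mode's flags.
; The line appears in a temporary WPB_LunaMonologue widget, removed after a short delay.
; A DoOnce blocks repeat triggers and resets only after a monologue, so interacting outside both modes leaves it locked.
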(event `self.ReceiveBeginPlay`
  (bind _asbp_lgamemode_first_person (cast `/Game/Luna/Blueprints/GameMode/BP_LGamemodeFirstPerson` (`GameplayStatics.GetGameMode`)))
  (set `self.As BP LGamemode First Person` _asbp_lgamemode_first_person))

(event `/Game/Luna/Input/BPI_Interactive.Interactive`
  (bind _as_bp_lgamemode_first_person (`self.As BP LGamemode First Person`))
  (`/Engine/EditorBlueprintResources/StandardMacros.DoOnce` false :!label _label
    (:`Completed`
      (if (`/Game/Luna/Blueprints/GameMode/BP_LGamemodeFirstPerson.SearchMode` _as_bp_lgamemode_first_person)
        (bind _returnvalue (`|CreateWidget` "/Game/Luna/UI/WPB_LunaMonologue.WPB_LunaMonologue_C" null (`self.Luna Says`)))
        (`UserWidget.AddToViewport` _returnvalue 0)
        (`KismetSystemLibrary.Delay` 3.0)
        (`Widget.RemoveFromParent` _returnvalue)
        (goto _label :!via `Reset`)
        (elif (`/Game/Luna/Blueprints/GameMode/BP_LGamemodeFirstPerson.EndingMode` _as_bp_lgamemode_first_person)
          (bind _returnvalue_2 (`|CreateWidget` "/Game/Luna/UI/WPB_LunaMonologue.WPB_LunaMonologue_C" null (`self.Luna Says_Ending`)))
          (`UserWidget.AddToViewport` _returnvalue_2 0)
          (`KismetSystemLibrary.Delay` 2.0)
          (`Widget.RemoveFromParent` _returnvalue_2)
          (goto _label :!via `Reset`))))))

(fn `UserConstructionScript`)