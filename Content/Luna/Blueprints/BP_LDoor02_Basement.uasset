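; Locked basement door that the Luna character can open once the first-person game mode reports a key.
; Interacting with the key removes the barricade once with a sound, then, if the overlap box has opened the gate, toggles a timeline-driven door swing with a creak.
; Without the key, it briefly shows an item-taking description widget, guarded by a DoOnce against repeats until removal.
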(event `/Game/Luna/Input/BPI_Interactive.Interactive`
  (if (`/Game/Luna/Blueprints/GameMode/BP_LGamemodeFirstPerson.HasKey` (stale `self.Box.OnComponentBeginOverlap` _asbp_lgamemode_first_person))
    (`self.LockOpens`)
    (`/Engine/EditorBlueprintResources/StandardMacros.Gate` true :!label _label
      (:`Exit`
        (`GameplayStatics.PlaySoundAtLocation` "/Game/Luna/Sounds/mixkit-creaky-door-open-195.mixkit-creaky-door-open-195" (`SceneComponent.K2_GetComponentLocation` (`self.Door_a`)) (struct) 1.0 1.0 0.0 null null null null)
        (`/Engine/EditorBlueprintResources/StandardMacros.FlipFlop`
          (:`A`
            (bind (_direction _alpha) (`Timeline|Timeline` :!label _label_2)
              (:`Update`
                (`SceneComponent.K2_SetRelativeRotation` (`self.Door_a`) (`KismetMathLibrary.RLerp` (struct) (struct :`Yaw` -90.0) _alpha) false false))))
          (:`B`
            (goto _label_2 :!via `Reverse`)))))
    (else
      (`/Engine/EditorBlueprintResources/StandardMacros.DoOnce` false :!label _label_3
        (:`Completed`
          (bind _returnvalue (`|CreateWidget` "/Game/Luna/UI/WPB_ItemTaking.WPB_ItemTaking_C" (`GameplayStatics.GetPlayerController` 0) (`self.Item Taking Desctiption`)))
          (`UserWidget.AddToViewport` _returnvalue 0)
          (`KismetSystemLibrary.Delay` 3.0)
          (`Widget.RemoveFromParent` _returnvalue)
          (goto _label_3 :!via `Reset`))))))

(event `self.Box.OnComponentBeginOverlap`
  (params (OverlappedComponent :type "PrimitiveComponent Object Reference") (OtherActor :type "Actor Object Reference") (OtherComp :type "PrimitiveComponent Object Reference") (OtherBodyIndex :type Integer) (bFromSweep :type Boolean) (SweepResult :type "HitResult Structure (by ref)"))
  (cast `/Game/Luna/Blueprints/BP_LunaCharacter` OtherActor)
  (bind _asbp_lgamemode_first_person (cast `/Game/Luna/Blueprints/GameMode/BP_LGamemodeFirstPerson` (`GameplayStatics.GetGameMode`)))
  (goto _label :!via `Open`))

(event `self.Box.OnComponentEndOverlap`
  (params (OverlappedComponent :type "PrimitiveComponent Object Reference") (OtherActor :type "Actor Object Reference") (OtherComp :type "PrimitiveComponent Object Reference") (OtherBodyIndex :type Integer))
  (cast `/Game/Luna/Blueprints/BP_LunaCharacter` OtherActor)
  (goto _label :!via `Close`))

(event `LockOpens`
  (`/Engine/EditorBlueprintResources/StandardMacros.DoOnce` false
    (:`Completed`
      (`GameplayStatics.PlaySoundAtLocation` "/Game/Luna/Sounds/mixkit-dropping-keys-in-the-floor-2839.mixkit-dropping-keys-in-the-floor-2839" (`SceneComponent.K2_GetComponentLocation` (`self.DoorBarricade_a`)) (struct) 1.0 1.0 0.0 null null null null)
      (`ActorComponent.K2_DestroyComponent` (`self.DoorBarricade_a`)))))

(fn `UserConstructionScript`)