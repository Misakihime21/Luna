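; BP_MissingMom is a trigger actor that shows a Luna monologue during the game's ending mode.
; BeginPlay caches the first-person game mode.
; When Luna's character enters the box while EndingMode is set, a DoOnce creates a monologue widget with the LunaSays text, displays it for four seconds, then removes it and destroys the actor.
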(event `self.ReceiveBeginPlay`
  (bind _asbp_lgamemode_first_person (cast `/Game/Luna/Blueprints/GameMode/BP_LGamemodeFirstPerson` (`GameplayStatics.GetGameMode`)))
  (set `self.As BP LGamemode First Person` _asbp_lgamemode_first_person))

(event `self.Box.OnComponentBeginOverlap`
  (params (OverlappedComponent :type "PrimitiveComponent Object Reference") (OtherActor :type "Actor Object Reference") (OtherComp :type "PrimitiveComponent Object Reference") (OtherBodyIndex :type Integer) (bFromSweep :type Boolean) (SweepResult :type "HitResult Structure (by ref)"))
  (cast `/Game/Luna/Blueprints/BP_LunaCharacter` OtherActor)
  (if (`/Game/Luna/Blueprints/GameMode/BP_LGamemodeFirstPerson.EndingMode` (`self.As BP LGamemode First Person`))
    (`/Engine/EditorBlueprintResources/StandardMacros.DoOnce` false
      (:`Completed`
        (bind _returnvalue (`|CreateWidget` "/Game/Luna/UI/WPB_LunaMonologue.WPB_LunaMonologue_C" null (`self.Luna Says`)))
        (`UserWidget.AddToViewport` _returnvalue 0)
        (`KismetSystemLibrary.Delay` 4.0)
        (`Widget.RemoveFromParent` _returnvalue)
        (`self.K2_DestroyActor`)))))

(fn `UserConstructionScript`)