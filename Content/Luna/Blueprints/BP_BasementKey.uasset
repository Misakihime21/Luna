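; BP_BasementKey is a pickup key that sets HasKey on the first-person game mode when the player interacts with it during SearchMode.
; A box overlap with BP_LunaCharacter shows a prompt widget, only in SearchMode, and hides it on exit.
; Interacting plays a key sound, removes the mesh and collision, shows an item-taking description widget for three seconds, then destroys the actor.
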(event `self.ReceiveBeginPlay`
  (bind _asbp_lgamemode_first_person (cast `/Game/Luna/Blueprints/GameMode/BP_LGamemodeFirstPerson` (`GameplayStatics.GetGameMode`)))
  (set `self.As BP LGamemode First Person` _asbp_lgamemode_first_person))

(event `/Game/Luna/Input/BPI_Interactive.Interactive`
  (bind _as_bp_lgamemode_first_person (`self.As BP LGamemode First Person`))
  (if (`/Game/Luna/Blueprints/GameMode/BP_LGamemodeFirstPerson.SearchMode` _as_bp_lgamemode_first_person)
    (`GameplayStatics.PlaySoundAtLocation` "/Game/Luna/Sounds/mixkit-dropping-keys-in-the-floor-2839.mixkit-dropping-keys-in-the-floor-2839" (`SceneComponent.K2_GetComponentLocation` (`self.Key_SM_Key`)) (struct) 1.0 1.0 0.0 null null null null)
    (set `/Game/Luna/Blueprints/GameMode/BP_LGamemodeFirstPerson.HasKey` true _as_bp_lgamemode_first_person)
    (bind _returnvalue (`|CreateWidget` "/Game/Luna/UI/WPB_ItemTaking.WPB_ItemTaking_C" null (`self.Item Taking Desctiption`)))
    (`ActorComponent.K2_DestroyComponent` (`self.Key_SM_Key`))
    (`ActorComponent.K2_DestroyComponent` (`self.BoxCollision`))
    (`UserWidget.AddToViewport` _returnvalue 0)
    (`KismetSystemLibrary.Delay` 3.0)
    (`Widget.RemoveFromParent` _returnvalue)
    (`self.K2_DestroyActor`)))

(event `self.BoxCollision.OnComponentBeginOverlap`
  (params (OverlappedComponent :type "PrimitiveComponent Object Reference") (OtherActor :type "Actor Object Reference") (OtherComp :type "PrimitiveComponent Object Reference") (OtherBodyIndex :type Integer) (bFromSweep :type Boolean) (SweepResult :type "HitResult Structure (by ref)"))
  (cast `/Game/Luna/Blueprints/BP_LunaCharacter` OtherActor)
  (if (`/Game/Luna/Blueprints/GameMode/BP_LGamemodeFirstPerson.SearchMode` (`self.As BP LGamemode First Person`))
    (`SceneComponent.SetHiddenInGame` (`self.Widget`) false false)))

(event `self.BoxCollision.OnComponentEndOverlap`
  (params (OverlappedComponent :type "PrimitiveComponent Object Reference") (OtherActor :type "Actor Object Reference") (OtherComp :type "PrimitiveComponent Object Reference") (OtherBodyIndex :type Integer))
  (cast `/Game/Luna/Blueprints/BP_LunaCharacter` OtherActor)
  (`SceneComponent.SetHiddenInGame` (`self.Widget`) true false))

(fn `UserConstructionScript`)